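; Base character for turn-based RPG battles, dispatching chosen actions to empty hooks meant for child overrides and tracking death and defending state.
; Attack and sauce-shot derive damage from cook-panel ingredients, while sauce-jar activates the chosen recipe; that value's range selects a quick-time event.
; The QTE is announced, started through AC_ActionManager, then polled each tick until the tap widget finishes.
; Targeting input and attack damage application are disconnected.
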(event OnBeginCursorOver(CapsuleComponent)
  (params (TouchedComponent :type Primitive%20Component%20Object%20Reference)))

(event OnEndCursorOver(CapsuleComponent)
  (params (TouchedComponent :type Primitive%20Component%20Object%20Reference)))

(event OnClicked(CapsuleComponent)
  (params (TouchedComponent :type Primitive%20Component%20Object%20Reference) (ButtonPressed :type Key%20Structure)))

(event Custom|QteEvent)

(event EventBeginPlay
  (Variables|/Script/Engine.PlayerController|SetbEnableMouseOverEvents (Game|GetPlayerController 0) true))

(event EventOnDamageReceived
  (params (Damage :type Float%20%28double-precision%29) (Critical :type Boolean) (IngredientsUsed :type Map%20of%20E_Ingridients%20Enums%20to%20Integers :default "NewEnumerator17")))

(event EventOnHealed
  (params (Amount :type Float%20%28double-precision%29) (RestoredMP :type Boolean)))

(event EventOnDeath
  (Variables|Battle|SetDead true)
  (Variables|/Game/Custom/Components/AC_CharacterBattleStats.AC_CharacterBattleStats_C|SetDefending (Variables|Default|GetAC_CharacterBattleStats) false))

(event Custom|ExecuteAction
  (params (ActionType :type E_ActionType%20Enum :default "NewEnumerator0") (SecondaryActionName :type Name))
  (bind _returnvalue (Game|GetPlayerController 0))
  (bind _returnvalue_2 (Actor|GetComponentbyClass _returnvalue "/Game/Custom/Components/AC_ActionManager.AC_ActionManager_C"))
  (switch Utilities|FlowControl|Switch|SwitchonE_ActionType ActionType
    (:NewEnumerator1
      (CallFunction|ExecuteActionAttack :!label _label)
      ;[0.15 0.15 0.15 0.5] Calculate QTE Diff Lev
      (bind _damanges (CallFunction|CalculateDMGSauceShot))
      (bind _qte_to_spawn (CallFunction|QTESpawn _damanges))
      (Variables|Default|SetQTEIndexToSpawn _qte_to_spawn)
      (bind _foundwidgets (Widget|GetAllWidgetsOfClass "/Game/Custom/Widgets/BattleWidgets/Widget_BattleInterface.Widget_BattleInterface_C" false :!label _label_2))
      (Utilities|IsValid (Utilities|Array|Get(acopy) _foundwidgets)
        (:Is%20Valid
          (Default|AnnounceQTE (Utilities|Array|Get(acopy) _foundwidgets) "Ready?")
          (Utilities|FlowControl|Delay 0.2)
          (Default|AnnounceQTE (Utilities|Array|Get(acopy) _foundwidgets) "Go!")
          (Utilities|FlowControl|Delay 0.2)
          ;[0.15 0.15 0.15 0.5] Create and check Qte event have succes
          (Default|SelectQTE (Actor|GetComponentbyClass (Game|GetPlayerController 0) "/Game/Custom/Components/AC_ActionManager.AC_ActionManager_C") (Variables|Default|GetQTEIndexToSpawn) 1.2 false "NewEnumerator17")
          (Variables|Default|SetQTEStart true)
          (bind _foundwidgets_2 (Widget|GetAllWidgetsOfClass "/Game/Custom/Widgets/BattleWidgets/Tap_Key_UI.Tap_Key_UI_C" false :!label _label_3))
          (Utilities|IsValid (Utilities|Array|Get(acopy) _foundwidgets_2 (Variables|Default|GetStartCheckIndex))
            (:Is%20Valid
              (Variables|/Script/Engine.PlayerController|SetbShowMouseCursor (Game|GetPlayerController 0) false)
              (if (Variables|/Game/Custom/Widgets/BattleWidgets/Tap_Key_UI.Tap_Key_UI_C|GetGo%20next%20frame (Utilities|Array|Get(acopy) _foundwidgets_2 (Variables|Default|GetStartCheckIndex)))
                (Variables|/Script/Engine.PlayerController|SetbShowMouseCursor (Game|GetPlayerController 0) true)
                (Class|WidgetSwitcher|SetActiveWidgetIndex (Variables|/Game/Custom/Widgets/BattleWidgets/Widget_ActionsPanel.Widget_ActionsPanel_C|GetWidgetSwitcher_Actions (Variables|/Game/Custom/Widgets/BattleWidgets/Widget_BattleInterface.Widget_BattleInterface_C|GetWidget_ActionsPanel (Variables|/Game/Custom/Components/AC_BattleManager.AC_BattleManager_C|GetBattleInterfaceReference (Variables|Default|GetBattleManagerReferences)))))
                (Variables|Default|SetQTEStart false)
                (else
                  (Utilities|FlowControl|DelayUntilNextTick)
                  (goto _label_3))))
            (:Is%20Not%20Valid
              (goto _label_3))))))
    (:NewEnumerator2
      (CallFunction|ExecuteActionDefend))
    (:NewEnumerator3
      (CallFunction|ExecuteActionItems SecondaryActionName))
    (:NewEnumerator4
      (CallFunction|ExecuteActionFlee))
    (:NewEnumerator5
      (CallFunction|ExecuteActionMagic SecondaryActionName))
    (:NewEnumerator6
      (CallFunction|ExecuteActionAbilities SecondaryActionName))
    (:NewEnumerator8
      (CallFunction|ExecuteActionPasta SecondaryActionName)
      (bind _dmg (Default|ActivateRecipe _returnvalue_2 (Variables|/Game/Custom/Components/AC_ActionManager.AC_ActionManager_C|GetChosenRecipe _returnvalue_2)))
      (bind _qte_to_spawn_2 (CallFunction|QTESpawn _dmg))
      (Variables|Default|SetQTEIndexToSpawn _qte_to_spawn_2)
      (goto _label_2))
    (:NewEnumerator10
      (goto _label))
    (:NewEnumerator11
      (CallFunction|ExecuteActionClearYourSelf))))

(event Custom|ExecuteAction_Attack
  ;[0.15 0.15 0.15 0.5] Will be overwritten in each child character
)

(event Custom|ExecuteAction_Defend
  ;[0.15 0.15 0.15 0.5] Will be overwritten in each child character
)

(event Custom|ExecuteAction_Items
  (params (SecondaryActionName :type Name))
  ;[0.15 0.15 0.15 0.5] Will be overwritten in each child character
)

(event Custom|ExecuteAction_Flee
  ;[0.15 0.15 0.15 0.5] Will be overwritten in each child character
)

(event Custom|ExecuteAction_Magic
  (params (SecondaryActionName :type Name))
  ;[0.15 0.15 0.15 0.5] Will be overwritten in each child character
)

(event Custom|ExecuteAction_Abilities
  (params (SecondaryActionName :type Name))
  ;[0.15 0.15 0.15 0.5] Will be overwritten in each child character
)

(event Custom|ExecuteAction_Pasta
  (params (PastaName :type Name))
  ;[0.15 0.15 0.15 0.5] Will be overwritten in each child character
)

(event Custom|ExecuteAction_ClearYourSelf
  ;[0.15 0.15 0.15 0.5] Will be overwritten in each child character
)

(fn ConstructionScript)

(fn ApplyAttackEffect
  (for _array_element (Variables|Battle|GetTargetedCharacters)
    (Utilities|IsValid _array_element)))

(fn PerformActionbyAI)

(fn CalculateDMGSauceShot
  (Variables|Default|SetDamage 0)
  (bind _foundwidgets (Widget|GetAllWidgetsOfClass "/Game/Custom/Widgets/BattleWidgets/Widget_Cook_Panel.Widget_Cook_Panel_C" false))
  (for _array_element _foundwidgets
    (bind _keys (Utilities|Map|Keys (Variables|/Game/Custom/Widgets/BattleWidgets/Widget_Cook_Panel.Widget_Cook_Panel_C|GetInUseIngridients _array_element)))
    (for _array_element_2 _keys
      (bind _returnvalue (Utilities|GetDataTableRow "/Game/Custom/DataTables/DT_Ingridients.DT_Ingridients" (Utilities|String|StringToName (Utilities|String|EnumtoString _array_element_2)))
        (:then
          (Variables|Default|SetDamage (+ (Variables|Default|GetDamage) (* (.Value (Utilities|Map|Find (Variables|/Game/Custom/Widgets/BattleWidgets/Widget_Cook_Panel.Widget_Cook_Panel_C|GetInUseIngridients _array_element) _array_element_2)) (.Dmg_Modifier (Utilities|Struct|BreakS_Ingridient _returnvalue))))))))
    (return (Math|Conversions|ToFloat(Integer) (Variables|Default|GetDamage)))))

(fn CalculateDMGSauceJar
  (Variables|Default|SetDamage 0)
  (bind _foundwidgets (Widget|GetAllWidgetsOfClass "/Game/Custom/Widgets/BattleWidgets/Widget_Cook_Panel.Widget_Cook_Panel_C" false))
  (for _array_element _foundwidgets
    (bind _keys (Utilities|Map|Keys (Variables|/Game/Custom/Widgets/BattleWidgets/Widget_Cook_Panel.Widget_Cook_Panel_C|GetInUseIngridients _array_element)))
    (for _array_element_2 _keys
      (bind _returnvalue (Utilities|GetDataTableRow "/Game/Custom/DataTables/DT_Ingridients.DT_Ingridients" (Utilities|String|StringToName (Utilities|String|EnumtoString _array_element_2)))
        (:then
          (Variables|Default|SetDamage (+ (Variables|Default|GetDamage) (* (.Value (Utilities|Map|Find (Variables|/Game/Custom/Widgets/BattleWidgets/Widget_Cook_Panel.Widget_Cook_Panel_C|GetInUseIngridients _array_element) _array_element_2)) (.Dmg_Modifier (Utilities|Struct|BreakS_Ingridient _returnvalue))))))))
    (Utilities|Map|Clear (Variables|/Game/Custom/Widgets/BattleWidgets/Widget_Cook_Panel.Widget_Cook_Panel_C|GetInUseIngridients _array_element))
    (Utilities|Array|Clear (Variables|/Game/Custom/Widgets/BattleWidgets/Widget_Cook_Panel.Widget_Cook_Panel_C|GetAInUseIngridients _array_element))
    (return (Math|Conversions|ToFloat(Integer) (Variables|Default|GetDamage)))))

(fn QTESpawn
  (params (Damanges :type Float%20%28double-precision%29))
  (Variables|Default|SetDamanges Damanges)
  (if (and (>= Damanges 480) (<= Damanges 599))
    (Variables|Default|SetQTEIndexToSpawn 4)
    (return (Variables|Default|GetQTEIndexToSpawn))
    (elif (and (>= Damanges 600) (<= Damanges 699))
      (Variables|Default|SetQTEIndexToSpawn 5)
      (return (Variables|Default|GetQTEIndexToSpawn))
      (elif (and (>= Damanges 700) (<= Damanges 800))
        (Variables|Default|SetQTEIndexToSpawn 6)
        (return (Variables|Default|GetQTEIndexToSpawn))))))

(fn IsDead
  (return (Variables|Battle|GetDead)))

(fn IsDefending
  (return (Variables|/Game/Custom/Components/AC_CharacterBattleStats.AC_CharacterBattleStats_C|GetDefending (Variables|Default|GetAC_CharacterBattleStats))))