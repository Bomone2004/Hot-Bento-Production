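; Farfalla enemy for turn-based, grid-based cooking combat, extending a parent enemy with its own action selection and movement.
; BeginPlay loads its DT_Enemies row, and action selection makes weighted random picks across two selection passes, overridden by sleep or betrayal.
; Movement simulates up to two knight-like hops on a five-wide grid, reserving free spots and carrying soiled state before MoveFromPosition teleports it.
; Front-row or blocked cases fall back to GoToRightTurnArray.
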(event EventBeginPlay
  (|CallParentFunction)
  (bind _returnvalue (Utilities|GetDataTableRow "/Game/Custom/DataTables/DT_Enemies.DT_Enemies" "BaseFarfalla")
    (:then
      (Variables|Default|SetsauceBarRegen (.CookingTimeRegen (Utilities|Struct|BreakS_Enemy _returnvalue)))
      (Variables|Default|SetWhatEnemyAmI (.EnemyHardcodedName (Utilities|Struct|BreakS_Enemy _returnvalue))))))

(event Collision|EventActorBeginOverlap
  (params (OtherActor :type Actor%20Object%20Reference))
  (|CallParentFunction OtherActor) ; This node is disabled and will not be called.\nDrag off pins to build functionality.
)

(event EventTick
  (params (DeltaSeconds :type Float%20%28single-precision%29))
  (|CallParentFunction DeltaSeconds) ; This node is disabled and will not be called.\nDrag off pins to build functionality.
)

(event EventOnSoiled
  (Variables|Default|SetisSoiled true)
  (bind _asgi_rpg (Utilities|Casting|CastToGI_RPG (Game|GetGameInstance)))
  (Variables|/Game/Custom/BP_EnemySpot.BP_EnemySpot_C|SetisEnemySoiled (.Value (Utilities|Map|Find (Variables|/Game/Custom/GI_RPG.GI_RPG_C|GetEnemySpotMap _asgi_rpg) (Variables|Default|GetsecondMovementIndex))) true))

(fn ConstructionScript
  (|CallParentFunction))

(fn TryBreakingPan
  (params (PointReference :type BP%20Enemy%20Spot%20Object%20Reference))
  (return true))

(fn RecoverSauceBar
  (bind _ac_characterbattlestats (Variables|Default|GetAC_CharacterBattleStats))
  (bind _returnvalue (Utilities|GetDataTableRow "/Game/Custom/DataTables/DT_Enemies.DT_Enemies" "BaseFarfalla")
    (:then
      (Variables|/Game/Custom/Components/AC_CharacterBattleStats.AC_CharacterBattleStats_C|SetCurrentHP _ac_characterbattlestats (Math|Float|Clamp(Float) (- (Variables|/Game/Custom/Components/AC_CharacterBattleStats.AC_CharacterBattleStats_C|GetCurrentHP _ac_characterbattlestats) (.SauceBarRegen (Utilities|Struct|BreakS_Enemy _returnvalue))) 0.0 (.Value (Utilities|Map|Find (Variables|/Game/Custom/Components/AC_CharacterBattleStats.AC_CharacterBattleStats_C|GetCharacterStats (Variables|Default|GetAC_CharacterBattleStats)) "NewEnumerator1"))))
      (Default|RefreshHP _ac_characterbattlestats))))

(fn StartRegeneration
  (|CallParentFunction))

(fn IsGettingCookedFunction
  (bind _output_get (Variables|Default|SetpoisonStack (- (Variables|Default|GetpoisonStack) 1)))
  (Development|PrintString (Utilities|String|Append "Turn before death for" (Utilities|GetDisplayName self) ": " (Utilities|String|ToString(Integer) _output_get)))
  (CallFunction|UpdateCookTime)
  (if (<= _output_get 0)
    (return true)
    (else
      (return false))))

(fn AttackPlayerFunction
  (|CallParentFunction))

(fn CreatePointArray
  (bind _secondmovementindex (Variables|Default|GetsecondMovementIndex))
  (bind _firstmovementindex (Variables|Default|GetfirstMovementIndex))
  (bind _firstmovementindex_2 (Variables|Default|GetfirstMovementIndex))
  (bind _firstmovementindex_3 (Variables|Default|GetfirstMovementIndex))
  (bind _firstmovementindex_4 (Variables|Default|GetfirstMovementIndex))
  (bind _firstmovementindex_5 (Variables|Default|GetfirstMovementIndex))
  (if (Variables|Default|GetfirstSimulationDone?)
    (if (<= _secondmovementindex 5)
      (CallFunction|GotoRightTurnArray)
      (else
        (Variables|Default|SetsecondTileIndexOccupied _secondmovementindex)
        (switch int (Math|Integer|%(Integer) (Variables|Default|GetsecondMovementIndex) 5)
          (:0
            (Variables|MoveFunction|SetMoveArray (Utilities|Array|MakeArray (- (Variables|Default|GetsecondMovementIndex) 7) (- (Variables|Default|GetsecondMovementIndex) 11))))
          (:1
            (Variables|MoveFunction|SetMoveArray (Utilities|Array|MakeArray (- (Variables|Default|GetsecondMovementIndex) 9) (- (Variables|Default|GetsecondMovementIndex) 3))))
          (:2
            (Variables|MoveFunction|SetMoveArray (Utilities|Array|MakeArray (- (Variables|Default|GetsecondMovementIndex) 3) (- (Variables|Default|GetsecondMovementIndex) 9) (- (Variables|Default|GetsecondMovementIndex) 11))))
          (:3
            (Variables|MoveFunction|SetMoveArray (Utilities|Array|MakeArray (- (Variables|Default|GetsecondMovementIndex) 3) (- (Variables|Default|GetsecondMovementIndex) 7) (- (Variables|Default|GetsecondMovementIndex) 9) (- (Variables|Default|GetsecondMovementIndex) 11))))
          (:4
            (Variables|MoveFunction|SetMoveArray (Utilities|Array|MakeArray (- (Variables|Default|GetsecondMovementIndex) 7) (- (Variables|Default|GetsecondMovementIndex) 9) (- (Variables|Default|GetsecondMovementIndex) 11)))))))
    (elif (<= _firstmovementindex_2 5)
      (CallFunction|GotoRightTurnArray)
      (else
        (Variables|Default|SetfirstTileIndexOccupied _firstmovementindex_2)
        (switch int (Math|Integer|%(Integer) (Variables|Default|GetfirstMovementIndex) 5)
          (:0
            (Variables|MoveFunction|SetMoveArray (Utilities|Array|MakeArray (- (Variables|Default|GetfirstMovementIndex) 7) (- (Variables|Default|GetfirstMovementIndex) 11))))
          (:1
            (Variables|MoveFunction|SetMoveArray (Utilities|Array|MakeArray (- _firstmovementindex_3 9) (- _firstmovementindex_3 3))))
          (:2
            (Variables|MoveFunction|SetMoveArray (Utilities|Array|MakeArray (- _firstmovementindex_4 3) (- _firstmovementindex_4 9) (- _firstmovementindex_4 11))))
          (:3
            (Variables|MoveFunction|SetMoveArray (Utilities|Array|MakeArray (- _firstmovementindex_5 3) (- _firstmovementindex_5 7) (- _firstmovementindex_5 9) (- _firstmovementindex_5 11))))
          (:4
            (Variables|MoveFunction|SetMoveArray (Utilities|Array|MakeArray (- _firstmovementindex 7) (- _firstmovementindex 9) (- _firstmovementindex 11)))))))))

(fn SelectActionfortheTurn
  (if (Variables|Default|GetsecondTurnSelection)
    (if (or (Variables|Default|GetisSleeping) (Variables|Default|GetbetrayON?))
      (Variables|Default|SetsecondSelectedAction "NewEnumerator4")
      (elif (Utilities|Enum|Equal(Enum) (Variables|Default|GetselectedAction) "NewEnumerator2")
        (switch int (Math|Random|RandomIntegerinRange 0 9)
          (:0
            (Variables|Default|SetsecondSelectedAction "NewEnumerator0" :!label _label))
          (:1
            (goto _label))
          (:2
            (goto _label))
          (:3
            (goto _label))
          (:4
            (goto _label))
          (:5
            (goto _label))
          (:6
            (goto _label))
          (:7
            (goto _label))
          (:8
            (goto _label))
          (:9
            (Variables|Default|SetsecondSelectedAction "NewEnumerator2")))
        (else
          (switch int (Math|Random|RandomIntegerinRange 0 9)
            (:0
              (Variables|Default|SetsecondSelectedAction "NewEnumerator0" :!label _label_2))
            (:1
              (goto _label_2))
            (:2
              (goto _label_2))
            (:3
              (goto _label_2))
            (:4
              (goto _label_2))
            (:5
              (goto _label_2))
            (:6
              (goto _label_2))
            (:7
              (goto _label_2))
            (:8
              (Variables|Default|SetsecondSelectedAction "NewEnumerator2" :!label _label_3))
            (:9
              (goto _label_3))))))
    (else
      (Variables|Default|SetsecondTurnSelection true)
      (if (or (Variables|Default|GetisSleeping) (Variables|Default|GetbetrayON?))
        (Variables|Default|SetselectedAction "NewEnumerator3")
        (else
          (switch int (Math|Random|RandomIntegerinRange 0 9)
            (:0
              (Variables|Default|SetsecondSelectedAction "NewEnumerator0" :!label _label_4))
            (:1
              (goto _label_4))
            (:2
              (goto _label_4))
            (:3
              (goto _label_4))
            (:4
              (goto _label_4))
            (:5
              (goto _label_4))
            (:6
              (goto _label_4))
            (:7
              (goto _label_4))
            (:8
              (Variables|Default|SetsecondSelectedAction "NewEnumerator2" :!label _label_5))
            (:9
              (goto _label_5))))))))

(fn SimulateMove
  (CallFunction|CreatePointArray)
  (bind _fail_ (CallFunction|SimulateMoveFunction))
  (Utilities|Array|Clear (Variables|MoveFunction|GetMoveArray))
  (if _fail_
    (CallFunction|GotoRightTurnArray)))

(fn SimulateMoveFunction
  (bind _movearray (Variables|MoveFunction|GetMoveArray))
  (bind _movearray_2 (Variables|MoveFunction|GetMoveArray))
  (bind _returnvalue (Utilities|Array|Length _movearray_2))
  (bind _returnvalue_2 (Utilities|Array|Length _movearray))
  (if (Variables|Default|GetfirstSimulationDone?)
    (if (== _returnvalue_2 0) :!label _label
      (return true)
      (else
        (bind _returnvalue_3 (Math|Random|RandomInteger _returnvalue_2))
        (if (< (Utilities|Array|Get(acopy) (Variables|MoveFunction|GetMoveArray) _returnvalue_3) 0)
          _
          (elif (.ReturnValue (Utilities|Map|Find (Variables|/Game/Custom/GI_RPG.GI_RPG_C|GetEnemySpotMap (Variables|Default|GetGameInstanceRef)) (Utilities|Array|Get(acopy) (Variables|MoveFunction|GetMoveArray) _returnvalue_3)))
            (if (Variables|/Game/Custom/BP_EnemySpot.BP_EnemySpot_C|GetisOccupied (.Value (Utilities|Map|Find (Variables|/Game/Custom/GI_RPG.GI_RPG_C|GetEnemySpotMap (Variables|Default|GetGameInstanceRef)) (Utilities|Array|Get(acopy) (Variables|MoveFunction|GetMoveArray) _returnvalue_3))))
              _
              (else
                (bind _output_get (Variables|MoveFunction|SetselectSpot (.Value (Utilities|Map|Find (Variables|/Game/Custom/GI_RPG.GI_RPG_C|GetEnemySpotMap (Variables|Default|GetGameInstanceRef)) (Utilities|Array|Get(acopy) (Variables|MoveFunction|GetMoveArray) _returnvalue_3)))))
                (Utilities|IsValid _output_get
                  (:Is%20Valid
                    (Variables|/Game/Custom/BP_EnemySpot.BP_EnemySpot_C|SetisOccupied _output_get true)
                    (Variables|/Game/Custom/BP_EnemySpot.BP_EnemySpot_C|SetisEnemySoiled _output_get (Variables|Default|GetisSoiled))
                    (Variables|/Game/Custom/BP_EnemySpot.BP_EnemySpot_C|SetisOccupied (.Value (Utilities|Map|Find (Variables|/Game/Custom/GI_RPG.GI_RPG_C|GetEnemySpotMap (Variables|Default|GetGameInstanceRef)) (Variables|Default|GetsecondMovementIndex))) false)
                    (Variables|/Game/Custom/BP_EnemySpot.BP_EnemySpot_C|SetisEnemySoiled (.Value (Utilities|Map|Find (Variables|/Game/Custom/GI_RPG.GI_RPG_C|GetEnemySpotMap (Variables|Default|GetGameInstanceRef)) (Variables|Default|GetsecondMovementIndex))) false)
                    (Variables|Default|SetsecondMovementIndex (Variables|/Game/Custom/BP_EnemySpot.BP_EnemySpot_C|GetSlotIndex (Variables|MoveFunction|GetselectSpot)))
                    (return false))
                  (:Is%20Not%20Valid
                    (return true)))))))
        (Utilities|Array|RemoveIndex (Variables|MoveFunction|GetMoveArray) _returnvalue_3)
        (goto _label)))
    (else
      (Variables|Default|SetfirstSimulationDone? true)
      (if (== _returnvalue 0) :!label _label_2
        (return true)
        (else
          (bind _returnvalue_4 (Math|Random|RandomInteger _returnvalue))
          (if (< (Utilities|Array|Get(acopy) (Variables|MoveFunction|GetMoveArray) _returnvalue_4) 0)
            _
            (elif (.ReturnValue (Utilities|Map|Find (Variables|/Game/Custom/GI_RPG.GI_RPG_C|GetEnemySpotMap (Variables|Default|GetGameInstanceRef)) (Utilities|Array|Get(acopy) (Variables|MoveFunction|GetMoveArray) _returnvalue_4)))
              (if (Variables|/Game/Custom/BP_EnemySpot.BP_EnemySpot_C|GetisOccupied (.Value (Utilities|Map|Find (Variables|/Game/Custom/GI_RPG.GI_RPG_C|GetEnemySpotMap (Variables|Default|GetGameInstanceRef)) (Utilities|Array|Get(acopy) (Variables|MoveFunction|GetMoveArray) _returnvalue_4))))
                _
                (else
                  (bind _output_get_2 (Variables|MoveFunction|SetselectSpot (.Value (Utilities|Map|Find (Variables|/Game/Custom/GI_RPG.GI_RPG_C|GetEnemySpotMap (Variables|Default|GetGameInstanceRef)) (Utilities|Array|Get(acopy) (Variables|MoveFunction|GetMoveArray) _returnvalue_4)))))
                  (Utilities|IsValid _output_get_2
                    (:Is%20Valid
                      (Variables|/Game/Custom/BP_EnemySpot.BP_EnemySpot_C|SetisOccupied _output_get_2 true)
                      (Variables|/Game/Custom/BP_EnemySpot.BP_EnemySpot_C|SetisEnemySoiled _output_get_2 (Variables|Default|GetisSoiled))
                      (Variables|/Game/Custom/BP_EnemySpot.BP_EnemySpot_C|SetisOccupied (.Value (Utilities|Map|Find (Variables|/Game/Custom/GI_RPG.GI_RPG_C|GetEnemySpotMap (Variables|Default|GetGameInstanceRef)) (Variables|Default|GetfirstMovementIndex))) false)
                      (Variables|/Game/Custom/BP_EnemySpot.BP_EnemySpot_C|SetisEnemySoiled (.Value (Utilities|Map|Find (Variables|/Game/Custom/GI_RPG.GI_RPG_C|GetEnemySpotMap (Variables|Default|GetGameInstanceRef)) (Variables|Default|GetfirstMovementIndex))) false)
                      (bind _output_get_3 (Variables|Default|SetfirstMovementIndex (Variables|/Game/Custom/BP_EnemySpot.BP_EnemySpot_C|GetSlotIndex (Variables|MoveFunction|GetselectSpot))))
                      (Variables|Default|SetsecondMovementIndex _output_get_3)
                      (return false))
                    (:Is%20Not%20Valid
                      (return true)))))))
          (Utilities|Array|RemoveIndex (Variables|MoveFunction|GetMoveArray) _returnvalue_4)
          (goto _label_2))))))

(fn MoveFunction
  (CallFunction|MovefromPosition))

(fn MovefromPosition
  (bind _secondmovementindex (Variables|Default|GetsecondMovementIndex))
  (bind _gameinstanceref (Variables|Default|GetGameInstanceRef))
  (bind _enemyspotmap (Variables|/Game/Custom/GI_RPG.GI_RPG_C|GetEnemySpotMap _gameinstanceref))
  (bind _value (Utilities|Map|Find _enemyspotmap _secondmovementindex))
  (bind _returnvalue (Transformation|GetActorTransform _value))
  (bind (_x _y) (Math|Vector|BreakVector (.location _returnvalue)))
  (if (Variables|Default|GetfirstMovementDone?)
    (Utilities|IsValid _value
      (:Is%20Valid
        (Transformation|SetActorLocation (Math|Vector|MakeVector _x _y (.z (Transformation|GetActorLocation))) false true)
        (Variables|/Game/Custom/BP_EnemySpot.BP_EnemySpot_C|SetenemyReference (.Value (Utilities|Map|Find (Variables|/Game/Custom/GI_RPG.GI_RPG_C|GetEnemySpotMap (Variables|Default|GetGameInstanceRef)) (Variables|Default|GetsecondTileIndexOccupied))) 0)
        (Variables|/Game/Custom/BP_EnemySpot.BP_EnemySpot_C|SetenemyReference _value self)
        (Default|StopShowing _value)
        (Variables|Default|SetfirstMovementIndex (Variables|Default|GetsecondMovementIndex)))
      (:Is%20Not%20Valid
        (Development|PrintString "")))
    (else
      (Variables|Default|SetfirstMovementDone? true)
      (Utilities|IsValid (.Value (Utilities|Map|Find (Variables|/Game/Custom/GI_RPG.GI_RPG_C|GetEnemySpotMap (Variables|Default|GetGameInstanceRef)) (Variables|Default|GetfirstMovementIndex)))
        (:Is%20Valid
          (Transformation|SetActorLocation (Math|Vector|MakeVector (.X (Math|Vector|BreakVector (.location (Transformation|GetActorTransform (.Value (Utilities|Map|Find (Variables|/Game/Custom/GI_RPG.GI_RPG_C|GetEnemySpotMap (Variables|Default|GetGameInstanceRef)) (Variables|Default|GetfirstMovementIndex))))))) (.Y (Math|Vector|BreakVector (.location (Transformation|GetActorTransform (.Value (Utilities|Map|Find (Variables|/Game/Custom/GI_RPG.GI_RPG_C|GetEnemySpotMap (Variables|Default|GetGameInstanceRef)) (Variables|Default|GetfirstMovementIndex))))))) (.z (Transformation|GetActorLocation))) false true)
          (Variables|/Game/Custom/BP_EnemySpot.BP_EnemySpot_C|SetenemyReference (.Value (Utilities|Map|Find (Variables|/Game/Custom/GI_RPG.GI_RPG_C|GetEnemySpotMap (Variables|Default|GetGameInstanceRef)) (Variables|Default|GetfirstTileIndexOccupied))) 0)
          (Variables|/Game/Custom/BP_EnemySpot.BP_EnemySpot_C|SetenemyReference (.Value (Utilities|Map|Find (Variables|/Game/Custom/GI_RPG.GI_RPG_C|GetEnemySpotMap (Variables|Default|GetGameInstanceRef)) (Variables|Default|GetfirstMovementIndex))) self)
          (Default|StopShowing (.Value (Utilities|Map|Find (Variables|/Game/Custom/GI_RPG.GI_RPG_C|GetEnemySpotMap (Variables|Default|GetGameInstanceRef)) (Variables|Default|GetfirstMovementIndex)))))
        (:Is%20Not%20Valid
          (Development|PrintString ""))))))